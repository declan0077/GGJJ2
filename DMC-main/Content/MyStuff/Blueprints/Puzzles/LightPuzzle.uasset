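; LightPuzzle is a puzzle light the player cycles through red, yellow and green by pressing E inside its overlap box.
; Each instance enables input on overlap, sets its colour via SwitchColour (also in the construction script) and flags IsOn when it matches CorrectColour.
; After every press it counts lit-correct LightPuzzle actors in the level; reaching RequiredAmount sets AllOn, which currently only prints debug text.
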(event OnComponentBeginOverlap(Box)
  (params (OverlappedComponent :type Primitive%20Component%20Object%20Reference) (OtherActor :type Actor%20Object%20Reference) (OtherComp :type Primitive%20Component%20Object%20Reference) (OtherBodyIndex :type Integer) (bFromSweep :type Boolean) (SweepResult :type Hit%20Result%20Structure%20%28by%20ref%29))
  ;[1 0 0.8158] Enable input
  (Input|EnableInput (Game|GetPlayerController 0)))

(event OnComponentEndOverlap(Box)
  (params (OverlappedComponent :type Primitive%20Component%20Object%20Reference) (OtherActor :type Actor%20Object%20Reference) (OtherComp :type Primitive%20Component%20Object%20Reference) (OtherBodyIndex :type Integer))
  ;[1 0 0.8158] Enable input
  (Input|DisableInput (Game|GetPlayerController 0)))

(event Custom|CheckIfAllOn
  ;[1 0 0.8173] Loops though all the lights and checks if they are all the correct light. If they all are correct the puzzle will be complete
  (bind _outactors (Actor|GetAllActorsOfClass "LightPuzzle_C"))
  (Variables|Default|SetOnCount 0)
  (for _array_element _outactors
    (Math|Integer|CompareInt (Math|Conversions|ToInteger(Boolean) (Variables|LightPuzzle_C|GetIsOn _array_element)) 1
      (:==
        (Variables|Default|SetOnCount (+ (Variables|Default|GetOnCount) 1))
        (if (>= (Variables|Default|GetOnCount) (Variables|Default|GetRequiredAmount))
          (Variables|Default|SetAllOn true)
          (Development|PrintString "AllOn")))))
  (if (Variables|Default|GetAllOn)
    (Development|PrintString "All on")))

(event Input|KeyboardEvents|E
  (params (Key :type Key%20Structure :default "None"))
  ;[1 0 0.848] Change colour of the light and check if its the correct light
  (:Pressed
    (bind _output_get (Variables|Default|SetLightInt (+ (Variables|Default|GetLightInt) 1)))
    (if (== _output_get 3)
      (bind _output_get_2 (Variables|Default|SetLightInt 0)))
    (CallFunction|SwitchColour _output_get_2)
    (if (== (Variables|Default|GetLightInt) (Variables|Default|GetCorrectColour))
      (Variables|Default|SetIsOn true)
      (else
        (Variables|Default|SetIsOn false)))
    (CallFunction|CheckifAllon)))

(fn ConstructionScript
  (CallFunction|SwitchColour (Variables|Default|GetLightInt)))

(fn SwitchColour
  (params (LightColour :type Integer))
  (bind _pointlight (Variables|Default|GetPointLight))
  ;[1 1 1] Switch colour based on Int
  (switch int LightColour
    (:0
      (Rendering|Components|Light|SetLightColor _pointlight "(R=1.000000,G=0.048928,B=0.000000,A=1.000000)" true))
    (:1
      (Rendering|Components|Light|SetLightColor _pointlight "(R=1.000000,G=0.871763,B=0.000000,A=1.000000)" true))
    (:2
      (Rendering|Components|Light|SetLightColor _pointlight "(R=0.012519,G=1.000000,B=0.000000,A=1.000000)" true))))